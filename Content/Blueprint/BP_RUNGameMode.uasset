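; Game mode for a runner game, with helpers that spawn floor tiles and a train.
; AddFloorTiles chains tiles by storing each new BP_FloorTile's attach transform as the next spawn point.
; AddTrain spawns BP_Train using the player mesh's relative transform, offset far along +X.
; BeginPlay is empty, and the graph that adds the train and ten starting tiles is disconnected, so it never runs.
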(event EventBeginPlay)

(fn ConstructionScript)

(fn AddFloorTiles
  (bind _returnvalue (Game|SpawnActorfromClass "/Game/Blueprint/Component/BP_FloorTile.BP_FloorTile_C" (Variables|Default|GetNextSpawnPoint) "Undefined" 0 0))
  (bind _asbp_floor_tile (Utilities|Casting|CastToBP_FloorTile _returnvalue))
  (bind _transform (Default|GetAttachTransform _asbp_floor_tile))
  (Variables|Default|SetNextSpawnPoint _transform))

(fn AddTrain
  (bind _asbp_running_man (Utilities|Casting|CastToBP_RunningMan (Game|GetPlayerCharacter 0)))
  (Game|SpawnActorfromClass "/Game/Blueprint/Component/BP_Train.BP_Train_C" (Math|Transform|MakeTransform (+ (.location (Transformation|GetRelativeTransform (Variables|/Script/Engine.Character|GetMesh _asbp_running_man))) "80000.000000,0,0") (.rotation (Transformation|GetRelativeTransform (Variables|/Script/Engine.Character|GetMesh _asbp_running_man))) (.scale (Transformation|GetRelativeTransform (Variables|/Script/Engine.Character|GetMesh _asbp_running_man)))) "AlwaysSpawn" 0 0))