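; BP_Soldier is an enemy soldier that gets thrown and explodes when it dies.
; On BeginPlay it caches the player's BP_RunningMan; Death flags it dead, disables capsule collision, makes Pantin ignore Pawns and starts the projection.
; A self-recalling Delay loop moves Pantin by lerped X/Y offsets until X reaches its death value.
; After a short pause, CharacterExplode spawns an explosion emitter and destroys the actor.
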(event Custom|Character%20is%20dead
  (bind _pantin (Variables|Default|GetPantin))
  (bind _returnvalue (Transformation|GetRelativeTransform _pantin))
  (if (> (Variables|Default|GetXPosition) (Variables|Default|GetXDeathPosition))
    (Transformation|SetRelativeTransform (Variables|Default|GetPantin) (Math|Transform|MakeTransform (+ (.location _returnvalue) (Math|Vector|MakeVector (Variables|Default|GetXPosition) (Variables|Default|GetYPosition) 1e+01)) (.rotation _returnvalue) "1.000000,1.000000,1.000000") false false :!label _label)
    (bind _output_get (Variables|Default|SetLerpDeath (Math|Float|Clamp(Float) (+ (Variables|Default|GetLerpDeath) 0.01))))
    (Variables|Default|SetYPosition (Math|Float|Lerp 0.0 (Variables|Default|GetYDeathPosition) _output_get))
    (Variables|Default|SetXPosition (Math|Float|Lerp -1.5e+02 (Variables|Default|GetXDeathPosition) _output_get))
    (Utilities|FlowControl|Delay 0.008)
    (CallFunction|ProjectingEvent)
    (goto _label)
    (else
      (Utilities|FlowControl|Delay 0.3)
      (CallFunction|CharacterExplode))))

(event Custom|ProjectingEvent
  (bind _pantin (Variables|Default|GetPantin))
  (bind _returnvalue (Transformation|GetRelativeTransform _pantin))
  (if (> (Variables|Default|GetXPosition) (Variables|Default|GetXDeathPosition))
    (Transformation|SetRelativeTransform (Variables|Default|GetPantin) (Math|Transform|MakeTransform (+ (.location _returnvalue) (Math|Vector|MakeVector (Variables|Default|GetXPosition) (Variables|Default|GetYPosition) 1e+01)) (.rotation _returnvalue) "1.000000,1.000000,1.000000") false false :!label _label)
    (bind _output_get (Variables|Default|SetLerpDeath (Math|Float|Clamp(Float) (+ (Variables|Default|GetLerpDeath) 0.01))))
    (Variables|Default|SetYPosition (Math|Float|Lerp 0.0 (Variables|Default|GetYDeathPosition) _output_get))
    (Variables|Default|SetXPosition (Math|Float|Lerp -1.5e+02 (Variables|Default|GetXDeathPosition) _output_get))
    (Utilities|FlowControl|Delay 0.008)
    (CallFunction|ProjectingEvent)
    (goto _label)
    (else
      (Utilities|FlowControl|Delay 0.3)
      (CallFunction|CharacterExplode))))

(event EventBeginPlay
  (CallFunction|GetBPCharacter))

(event EventTick
  (params (DeltaSeconds :type Float%20%28single-precision%29)))

(fn ConstructionScript)

(fn Death
  (Variables|Default|SetIsDead true)
  (CallFunction|CharacterIsDead)
  (Collision|SetCollisionResponsetoChannel (Variables|Default|GetPantin) "ECC_Pawn" "ECR_Ignore")
  (Collision|SetCollisionEnabled (Variables|Default|GetCapsule) "NoCollision"))

(fn GetBPCharacter
  (bind _asbp_running_man (Utilities|Casting|CastToBP_RunningMan (Game|Player|GetPlayerPawn 0)))
  (Variables|Default|SetAs%20BP%20Running%20Man _asbp_running_man))

(fn CharacterExplode
  (bind _pantin (Variables|Default|GetPantin))
  (bind _returnvalue (Transformation|GetWorldTransform _pantin))
  (Effects|SpawnEmitteratLocation "/Game/StarterContent/Particles/P_Explosion.P_Explosion" (.location _returnvalue) (.rotation _returnvalue) "2.000000,2.000000,2.000000")
  (Actor|DestroyActor))