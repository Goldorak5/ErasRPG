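; BP_SoldierSmall is an enemy soldier that repeatedly spawns an actor, likely a projectile, from its Arrow component.
; BeginPlay runs a delayed loop that spawns at a fixed interval until IsDead is set.
; On death, Tick switches the Pantin mesh to Animation Blueprint mode and destroys the Gun, once.
; The Box overlap filters for BP_RunningMan but triggers nothing after its DoOnce.
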(event OnComponentBeginOverlap(Box)
  (params (OverlappedComponent :type Primitive%20Component%20Object%20Reference) (OtherActor :type Actor%20Object%20Reference) (OtherComp :type Primitive%20Component%20Object%20Reference) (OtherBodyIndex :type Integer) (bFromSweep :type Boolean) (SweepResult :type Hit%20Result%20Structure%20%28by%20ref%29))
  (Utilities|Casting|CastToBP_RunningMan OtherActor)
  (Utilities|FlowControl|DoOnce false))

(event EventBeginPlay
  (|CallParentFunction)
  (Game|SpawnActorfromClass "/Game/Blueprint/Character/RunningMan/projectile/BP_Projectile.BP_Projectile_C" (Transformation|GetWorldTransform (Variables|Default|GetArrow)) "AlwaysSpawn" 0 0 :!label _label)
  (Utilities|FlowControl|Delay 1.2)
  (if (not (Variables|Default|GetIsDead))
    (goto _label)))

(event EventTick
  (params (DeltaSeconds :type Float%20%28single-precision%29))
  (|CallParentFunction 0.0)
  (if (Variables|Default|GetIsDead)
    (Utilities|FlowControl|DoOnce false
      (:Completed
        (Components|Animation|SetAnimationMode (Variables|Default|GetPantin) "AnimationBlueprint")
        (Components|DestroyComponent (Variables|Default|GetGun))))))

(fn ConstructionScript
  (|CallParentFunction))