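; Medium soldier enemy that swings a great sword when the BP_RunningMan character comes within range.
; Two trigger boxes, Box and RightBox, play the left and right sword animations respectively on the Pantin component.
; Each trigger fires only once through its own DoOnce, which is never reset here.
; BeginPlay, Tick, actor overlap and construction only forward to the parent class.
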(event OnComponentBeginOverlap(Box)
  (params (OverlappedComponent :type Primitive%20Component%20Object%20Reference) (OtherActor :type Actor%20Object%20Reference) (OtherComp :type Primitive%20Component%20Object%20Reference) (OtherBodyIndex :type Integer) (bFromSweep :type Boolean) (SweepResult :type Hit%20Result%20Structure%20%28by%20ref%29))
  (Utilities|Casting|CastToBP_RunningMan OtherActor)
  (Utilities|FlowControl|DoOnce false
    (:Completed
      (Components|Animation|PlayAnimation (Variables|Default|GetPantin) "/Game/Blueprint/Character/Enemy/Soldier/MediumSoldier/GreatSwordLeft.GreatSwordLeft" false))))

(event OnComponentBeginOverlap(RightBox)
  (params (OverlappedComponent :type Primitive%20Component%20Object%20Reference) (OtherActor :type Actor%20Object%20Reference) (OtherComp :type Primitive%20Component%20Object%20Reference) (OtherBodyIndex :type Integer) (bFromSweep :type Boolean) (SweepResult :type Hit%20Result%20Structure%20%28by%20ref%29))
  (Utilities|Casting|CastToBP_RunningMan OtherActor)
  (Utilities|FlowControl|DoOnce false
    (:Completed
      (Components|Animation|PlayAnimation (Variables|Default|GetPantin) "/Game/Blueprint/Character/Enemy/Soldier/MediumSoldier/GreatSwordRight.GreatSwordRight" false))))

(event EventBeginPlay
  (|CallParentFunction))

(event Collision|EventActorBeginOverlap
  (params (OtherActor :type Actor%20Object%20Reference))
  (|CallParentFunction OtherActor))

(event EventTick
  (params (DeltaSeconds :type Float%20%28single-precision%29))
  (|CallParentFunction DeltaSeconds))

(fn ConstructionScript
  (|CallParentFunction))