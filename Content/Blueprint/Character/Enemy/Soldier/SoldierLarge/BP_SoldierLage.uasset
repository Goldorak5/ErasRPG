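; BP_SoldierLage is a large soldier enemy that fires a short missile salvo when BP_RunningMan enters its trigger box.
; A DoOnce limits the attack to a single salvo: two BP_ProjectileMissile actors spawn at the Arrow's transform, a brief delay apart.
; BeginPlay caches three scene component transforms as landing points, which this graph never reads.
; Other begin-play, tick and actor overlap behavior comes from the parent class.
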(event OnComponentBeginOverlap(Box)
  (params (OverlappedComponent :type Primitive%20Component%20Object%20Reference) (OtherActor :type Actor%20Object%20Reference) (OtherComp :type Primitive%20Component%20Object%20Reference) (OtherBodyIndex :type Integer) (bFromSweep :type Boolean) (SweepResult :type Hit%20Result%20Structure%20%28by%20ref%29))
  (Utilities|Casting|CastToBP_RunningMan OtherActor)
  (Utilities|FlowControl|Sequence
    (:then_0
      (Utilities|FlowControl|DoOnce false
        (:Completed
          (Game|SpawnActorfromClass "/Game/Blueprint/Character/Enemy/Soldier/SoldierLarge/BP_ProjectileMissile.BP_ProjectileMissile_C" (Transformation|GetWorldTransform (Variables|Default|GetArrow)) "Undefined" 0 0)
          (Utilities|FlowControl|Delay 0.2)
          (Game|SpawnActorfromClass "/Game/Blueprint/Character/Enemy/Soldier/SoldierLarge/BP_ProjectileMissile.BP_ProjectileMissile_C" (Transformation|GetWorldTransform (Variables|Default|GetArrow)) "Undefined" 0 0))))))

(event EventBeginPlay
  (|CallParentFunction)
  (CallFunction|SetTransformLandingpoint))

(event Collision|EventActorBeginOverlap
  (params (OtherActor :type Actor%20Object%20Reference))
  (|CallParentFunction OtherActor))

(event EventTick
  (params (DeltaSeconds :type Float%20%28single-precision%29))
  (|CallParentFunction DeltaSeconds))

(fn ConstructionScript
  (|CallParentFunction))

(fn SetTransformLandingpoint
  (Variables|Default|Setarrow3Tranform (Utilities|Array|MakeArray (Transformation|GetWorldTransform (Variables|Default|GetScene1)) (Transformation|GetWorldTransform (Variables|Default|GetScene2)) (Transformation|GetWorldTransform (Variables|Default|GetScene3)))))