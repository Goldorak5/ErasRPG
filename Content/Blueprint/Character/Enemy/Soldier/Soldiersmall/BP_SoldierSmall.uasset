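; Small soldier enemy that automatically fires projectiles until it dies, extending parent behavior.
; BeginPlay starts a delay loop that spawns BP_Projectile at the Arrow component's transform at a fixed interval while IsDead is false.
; Tick polls IsDead and, through a DoOnce on death, switches the Pantin mesh to Animation Blueprint mode and destroys the Gun component.
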(event EventBeginPlay
  (|CallParentFunction)
  (Game|SpawnActorfromClass "/Game/Blueprint/Character/Enemy/Soldier/Soldiersmall/projectile/BP_Projectile.BP_Projectile_C" (Transformation|GetWorldTransform (Variables|Default|GetArrow)) "AlwaysSpawn" 0 0 :!label _label)
  (Utilities|FlowControl|Delay 1.2)
  (if (not (Variables|Default|GetIsDead))
    (goto _label)))

(event EventTick
  (params (DeltaSeconds :type Float%20%28single-precision%29))
  (|CallParentFunction 0.0)
  (if (Variables|Default|GetIsDead)
    (Utilities|FlowControl|DoOnce false
      (:Completed
        (Components|Animation|SetAnimationMode (Variables|Default|GetPantin) "AnimationBlueprint")
        (Components|DestroyComponent (Variables|Default|GetGun))))))

(fn ConstructionScript
  (|CallParentFunction))