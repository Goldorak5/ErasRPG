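; BP_Projectile is a small-soldier enemy projectile with a one-second lifespan that redirects when it hits a shielded player.
; On box overlap with a shielded BP_RunningMan, it enables homing on its Target component and re-aims its velocity toward that component's relative location at initial speed.
; Overlaps with an unshielded player trigger no logic here, and RotateToTarget is an empty event.
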(event OnComponentBeginOverlap(Box)
  (params (OverlappedComponent :type Primitive%20Component%20Object%20Reference) (OtherActor :type Actor%20Object%20Reference) (OtherComp :type Primitive%20Component%20Object%20Reference) (OtherBodyIndex :type Integer) (bFromSweep :type Boolean) (SweepResult :type Hit%20Result%20Structure%20%28by%20ref%29))
  (bind _projectilemovement (Variables|Default|GetProjectileMovement))
  (bind _asbp_running_man (Utilities|Casting|CastToBP_RunningMan OtherActor))
  (if (Variables|/Game/Blueprint/Character/RunningMan/BP_RunningMan.BP_RunningMan_C|GetIsShielded _asbp_running_man)
    (bind _target (Variables|Target|GetTarget)
      (:then
        (Variables|/Script/Engine.ProjectileMovementComponent|SetbIsHomingProjectile _projectilemovement true)
        (Variables|/Script/Engine.ProjectileMovementComponent|SetHomingTargetComponent _projectilemovement _target)
        (bind _target_2 (Variables|Target|GetTarget)
          (:then
            (Variables|/Script/Engine.MovementComponent|SetVelocity (Variables|Default|GetProjectileMovement) (* (Math|Vector|GetUnitDirection(Vector) (Transformation|GetActorLocation) (Variables|/Script/Engine.SceneComponent|GetRelativeLocation _target_2)) (Variables|/Script/Engine.ProjectileMovementComponent|GetInitialSpeed (Variables|Default|GetProjectileMovement)))))
          (:else)))
      (:else))))

(event Custom|RotateToTarget)

(event EventBeginPlay
  (Actor|SetLifeSpan 1.0))

(fn ConstructionScript)