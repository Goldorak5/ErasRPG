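; BP_Door is a door that BP_RunningMan can push away, after which it moves, explodes and is destroyed.
; Tick box-traces along negative X and activates the Door component when it hits the player while PushingDoor is set.
; Activation starts ControleDoor, a self-calling Delay loop that adds per-axis move and spin offsets through DoorMovement.
; LerpSpeed only counts progress; at its limit the door hides, spawns P_Explosion and destroys the actor.
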(event OnComponentActivated(Door)
  (params (Component :type Actor%20Component%20Object%20Reference) (bReset :type Boolean))
  (if (== (Variables|Default|GetLerpSpeed) 1.0)
    (Rendering|SetVisibility (Variables|Default|GetDoor) false false)
    (Effects|SpawnEmitteratLocation "/Game/StarterContent/Particles/P_Explosion.P_Explosion" (Variables|/Script/Engine.SceneComponent|GetRelativeLocation (Variables|Default|GetDoor)))
    (Utilities|FlowControl|Delay 0.2)
    (Actor|DestroyActor)
    (else
      (bind _output_get (Variables|Default|SetLerpSpeed (Math|Float|Clamp(Float) (+ (Variables|Default|GetLerpSpeed) 0.02))))
      (bind (_forwardspeed _sidespeed _upspeed _rotationx _rotationy _rotaionz _scalevalue) (CallFunction|DoorMovement _output_get))
      (Transformation|SetRelativeTransform (Variables|Default|GetDoor) (Math|Transform|MakeTransform (Math|Vector|MakeVector _forwardspeed _sidespeed _upspeed) (Math|Rotator|MakeRotator _rotationx _rotationy _rotaionz) _scalevalue) false false)
      (Utilities|FlowControl|Delay 0.0001)
      (CallFunction|ControleDoor))))

(event Custom|ControleDoor
  (if (== (Variables|Default|GetLerpSpeed) 1.0)
    (Rendering|SetVisibility (Variables|Default|GetDoor) false false)
    (Effects|SpawnEmitteratLocation "/Game/StarterContent/Particles/P_Explosion.P_Explosion" (Variables|/Script/Engine.SceneComponent|GetRelativeLocation (Variables|Default|GetDoor)))
    (Utilities|FlowControl|Delay 0.2)
    (Actor|DestroyActor)
    (else
      (bind _output_get (Variables|Default|SetLerpSpeed (Math|Float|Clamp(Float) (+ (Variables|Default|GetLerpSpeed) 0.02))))
      (bind (_forwardspeed _sidespeed _upspeed _rotationx _rotationy _rotaionz _scalevalue) (CallFunction|DoorMovement _output_get))
      (Transformation|SetRelativeTransform (Variables|Default|GetDoor) (Math|Transform|MakeTransform (Math|Vector|MakeVector _forwardspeed _sidespeed _upspeed) (Math|Rotator|MakeRotator _rotationx _rotationy _rotaionz) _scalevalue) false false)
      (Utilities|FlowControl|Delay 0.0001)
      (CallFunction|ControleDoor))))

(event EventBeginPlay
  (bind _asbp_running_man (Utilities|Casting|CastToBP_RunningMan (Game|GetPlayerCharacter 0)))
  (bind _output_get (Variables|Default|SetAs%20BP%20Running%20Man _asbp_running_man)))

(event EventTick
  (params (DeltaSeconds :type Float%20%28single-precision%29))
  (bind _returnvalue (Transformation|GetActorLocation))
  (bind _box (Variables|Default|GetBox))
  (bind _outhit (Class|KismetSystemLibrary|BoxTraceSingleforObjects _returnvalue (- _returnvalue "500.000000,0,0") (Components|Box|GetScaledBoxExtent _box) (.rotation (Transformation|GetWorldTransform _box)) (Variables|Default|GetObject%20Types) false 0 "None" true))
  (Utilities|Casting|CastToBP_RunningMan (.hitactor _outhit))
  (if (Variables|/Game/Blueprint/Character/RunningMan/BP_RunningMan.BP_RunningMan_C|GetPushingDoor (stale EventBeginPlay _output_get))
    (Components|Activation|Activate (Variables|Default|GetDoor) false)))

(fn ConstructionScript)

(fn DoorMovement
  (params (Lerp :type Float%20%28double-precision%29))
  (bind _door (Variables|Default|GetDoor))
  (bind _returnvalue (Transformation|GetRelativeTransform _door))
  (bind _relativerotation (Variables|/Script/Engine.SceneComponent|GetRelativeRotation _door))
  (return (+ (.x (.location _returnvalue)) (Variables|Default|GetForwardSpeed)) (+ (.y (.location _returnvalue)) (Variables|Default|GetSideSpeed)) (+ (.z (.location _returnvalue)) (Variables|Default|GetUpSpeed)) (+ (.roll _relativerotation) (Variables|Default|GetRotationSpeedX)) (+ (.pitch _relativerotation) (Variables|Default|GetRotationSpeedY)) (+ (.yaw _relativerotation) (Variables|Default|GetRotationSpeedZ)) (.scale _returnvalue)))