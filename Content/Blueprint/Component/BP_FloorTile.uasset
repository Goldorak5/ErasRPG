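; BP_FloorTile is a floor segment for an endless-runner track, exposing an attach-point transform.
; When BP_RunningMan enters its spawn zone, it has BP_RUNGameMode add floor tiles, then destroys itself after a short delay.
; Random soldier spawning at center, right or left points exists but is disconnected from the construction script.
; AccelerationRunningMan is called on overlap, but its speed-doubling step is unwired, so speed is unchanged.
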(event OnComponentBeginOverlap(SpawZone)
  (params (OverlappedComponent :type Primitive%20Component%20Object%20Reference) (OtherActor :type Actor%20Object%20Reference) (OtherComp :type Primitive%20Component%20Object%20Reference) (OtherBodyIndex :type Integer) (bFromSweep :type Boolean) (SweepResult :type Hit%20Result%20Structure%20%28by%20ref%29))
  (Utilities|Casting|CastToBP_RunningMan OtherActor)
  (bind _asbp_rungame_mode (Utilities|Casting|CastToBP_RUNGameMode (Game|GetGameMode)))
  (Default|AddFloorTiles _asbp_rungame_mode)
  (CallFunction|AccelerationRunningMan)
  (Utilities|FlowControl|Delay 3.0)
  (Actor|DestroyActor))

(event EventBeginPlay)

(event Collision|EventActorBeginOverlap
  (params (OtherActor :type Actor%20Object%20Reference)))

(event EventTick
  (params (DeltaSeconds :type Float%20%28single-precision%29)))

(fn ConstructionScript)

(fn GetAttachTransform
  (return (Transformation|GetWorldTransform (Variables|Default|GetAttachPoint))))

(fn SetSpawningpoints
  (bind _center (Variables|Default|GetCenter))
  (bind _right (Variables|Default|GetRight))
  (bind _left (Variables|Default|GetLeft))
  (bind _returnvalue (Transformation|GetRelativeTransform _center))
  (bind _returnvalue_2 (Transformation|GetRelativeTransform _right))
  (bind _returnvalue_3 (Transformation|GetRelativeTransform _left))
  (Variables|Default|SetSpawningPoints (Utilities|Array|MakeArray (Math|Transform|MakeTransform (.location _returnvalue) (.rotation _returnvalue) "1.000000,1.000000,1.000000") (Math|Transform|MakeTransform (.location _returnvalue_2) (.rotation _returnvalue_2) "1.000000,1.000000,1.000000") (Math|Transform|MakeTransform (.location _returnvalue_3) (.rotation _returnvalue_3) "1.000000,1.000000,1.000000"))))

(fn SpawnSoldierSmall
  (bind _spawningpoints (Variables|Default|GetSpawningPoints))
  (AddComponent|AddChildActorComponent false (Utilities|Array|Get(acopy) _spawningpoints (Math|Random|RandomIntegerinRange 0 (Utilities|Array|LastIndex _spawningpoints)))))

(fn AccelerationRunningMan
  (Utilities|Casting|CastToBP_RunningMan (Game|GetPlayerCharacter 0)))

(fn SpawnSoldierMedium
  (bind _spawningpoints (Variables|Default|GetSpawningPoints))
  (AddComponent|AddChildActorComponent false (Utilities|Array|Get(acopy) _spawningpoints (Math|Random|RandomIntegerinRange 0 (Utilities|Array|LastIndex _spawningpoints)))))

(fn SpawnSoldierLarge
  (bind _spawningpoints (Variables|Default|GetSpawningPoints))
  (AddComponent|AddChildActorComponent false (Utilities|Array|Get(acopy) _spawningpoints (Math|Random|RandomIntegerinRange 0 (Utilities|Array|LastIndex _spawningpoints)))))