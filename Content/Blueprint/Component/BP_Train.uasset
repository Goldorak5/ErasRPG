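; BP_Train is a train obstacle or vehicle actor that slides along world X.
; Every Tick, TrainMovement offsets the Train component by TrainSpeed without delta-time scaling or sweep, so speed depends on frame rate.
; SpawnTrain, not called within this file, spawns another BP_Train near world X 1000, adding only the BP_RunningMan mesh's forward vector, not its location, and copying that mesh's relative rotation and scale.
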(event EventBeginPlay)

(event EventTick
  (params (DeltaSeconds :type Float%20%28single-precision%29))
  (CallFunction|TrainMovement))

(fn ConstructionScript)

(fn SpawnTrain
  (bind _asbp_running_man (Utilities|Casting|CastToBP_RunningMan (Game|GetPlayerCharacter 0)))
  (Game|SpawnActorfromClass "BP_Train_C" (Math|Transform|MakeTransform (+ (Math|Vector|GetForwardVector (Variables|/Script/Engine.Character|GetMesh _asbp_running_man)) "1000.000000,0,0") (.rotation (Transformation|GetRelativeTransform (Variables|/Script/Engine.Character|GetMesh _asbp_running_man))) (.scale (Transformation|GetRelativeTransform (Variables|/Script/Engine.Character|GetMesh _asbp_running_man)))) "AlwaysSpawn" 0 0))

(fn TrainMovement
  (bind _train (Variables|Default|GetTrain))
  (Transformation|SetWorldLocation _train (+ (Transformation|GetWorldLocation _train) (* "1.000000,0,0" (Variables|Default|GetTrainSpeed))) false false))