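; BP_TriggerBoxPause is a one-shot trigger volume that pauses the game and shows a start screen when BP_RunningMan enters it.
; On overlap it stores the character, enables its player input, pauses the game and adds a WD_StartGame widget to the viewport.
; Tick polls the character's PauseGame flag; once false, it removes the widget, unpauses the game and destroys the trigger.
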(event OnComponentBeginOverlap(Box)
  (params (OverlappedComponent :type Primitive%20Component%20Object%20Reference) (OtherActor :type Actor%20Object%20Reference) (OtherComp :type Primitive%20Component%20Object%20Reference) (OtherBodyIndex :type Integer) (bFromSweep :type Boolean) (SweepResult :type Hit%20Result%20Structure%20%28by%20ref%29))
  (bind _asbp_running_man (Utilities|Casting|CastToBP_RunningMan OtherActor))
  (Variables|Default|SetAs%20BP%20Running%20Man _asbp_running_man)
  (Input|EnableInput _asbp_running_man (Game|GetPlayerController 0))
  (Game|SetGamePaused true)
  (bind _returnvalue (UserInterface|CreateWidget "/Game/Blueprint/Character/RunningMan/WD_StartGame.WD_StartGame_C"))
  (UserInterface|Viewport|AddtoViewport _returnvalue 0))

(event EventTick
  (params (DeltaSeconds :type Float%20%28single-precision%29))
  (bind _as_bp_running_man (Variables|Default|GetAs%20BP%20Running%20Man)
    (:then
      (if (not (Variables|/Game/Blueprint/Character/RunningMan/BP_RunningMan.BP_RunningMan_C|GetPauseGame _as_bp_running_man))
        (Widget|RemovefromParent (stale OnComponentBeginOverlap(Box) _returnvalue))
        (Game|SetGamePaused (Variables|/Game/Blueprint/Character/RunningMan/BP_RunningMan.BP_RunningMan_C|GetPauseGame _as_bp_running_man))
        (Actor|DestroyActor)))
    (:else)))

(fn ConstructionScript)