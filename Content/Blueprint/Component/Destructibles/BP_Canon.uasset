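; Destructible cannon turret that targets BP_RunningMan and is destroyed by the player's fully charged projection.
; PawnSensing shows a warning, aims at the player and fires a one-time delayed BP_Laser, restoring its original transform when the player is closer than the deactivation distance.
; A per-tick box trace detects the projecting player and triggers death: physics simulation, Chaos strain and velocity fields, Niagara fire, then actor destruction.
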(event OnSeePawn(PawnSensing)
  (params (Pawn :type Pawn%20Object%20Reference))
  (bind _asbp_running_man (Utilities|Casting|CastToBP_RunningMan Pawn))
  (if (>= (Math|Vector|Distance(Vector) (Transformation|GetActorLocation) (Transformation|GetActorLocation _asbp_running_man)) (Variables|Default|GetDistanceToDeactivateTurret))
    (Rendering|SetVisibility (Variables|Default|GetAvertissement) true false)
    (Transformation|SetActorRotation (Math|Rotator|FindLookatRotation (Transformation|GetActorLocation) (- (Transformation|GetWorldLocation (Variables|/Script/Engine.Actor|GetRootComponent _asbp_running_man)) (Variables|Default|GetTargetLockAjust))))
    (Utilities|FlowControl|DoOnce false
      (:Completed
        (Utilities|Time|SetTimerbyEvent (delegate Custom|Shoot) 1.0)))
    (else
      (Transformation|SetActorTransform (Variables|Default|GetActorTransformOrigin)))))

(event Custom|CanonDeath
  (Physics|SetSimulatePhysics (Variables|Default|GetCanon) true)
  (CallFunction|CreateField)
  (Utilities|FlowControl|Delay 0.4)
  (CallFunction|SpawnNiagara)
  (Actor|DestroyActor))

(event Custom|Shoot
  (Game|SpawnActorfromClass "/Game/Blueprint/Component/Destructibles/BP_Laser.BP_Laser_C" (Transformation|GetWorldTransform (Variables|Default|GetArrow)) "Undefined" 0 0))

(event EventBeginPlay
  (bind _asbp_running_man (Utilities|Casting|CastToBP_RunningMan (Game|Player|GetPlayerPawn 0)))
  (Variables|Default|SetAs%20BP%20Running%20Man _asbp_running_man)
  (Variables|Default|SetActorTransformOrigin (Transformation|GetActorTransform)))

(event EventTick
  (params (DeltaSeconds :type Float%20%28single-precision%29))
  (bind _outhit_hitactor (CallFunction|BoxTraceDetectRunningMan))
  (bind _asbp_running_man (Utilities|Casting|CastToBP_RunningMan _outhit_hitactor))
  (if (and (Variables|/Game/Blueprint/Character/RunningMan/BP_RunningMan.BP_RunningMan_C|GetChargingProjectionLvlMax _asbp_running_man) (Variables|/Game/Blueprint/Character/RunningMan/BP_RunningMan.BP_RunningMan_C|GetActivateProjection _asbp_running_man))
    (Utilities|FlowControl|DoOnce false
      (:Completed
        (Physics|SetSimulatePhysics (Variables|Default|GetCanon) true)
        (CallFunction|CreateField)
        (Utilities|FlowControl|Delay 0.4)
        (CallFunction|SpawnNiagara)
        (Actor|DestroyActor)))))

(fn ConstructionScript)

(fn CreateField
  (bind _force (Variables|Default|GetForce))
  (bind _force_2 (Variables|Default|GetForce))
  (bind _returnvalue (Transformation|GetWorldLocation _force_2))
  (Class|FieldSystemComponent|ApplyPhysicsField _force true "Field_ExternalClusterStrain" 0 (Field|SetRadialFalloff (Variables|Default|GetRadialFalloff) 1e+04 1.0 1.0 0.0 5e+02 _returnvalue "Field_Falloff_Linear"))
  (Class|FieldSystemComponent|ApplyPhysicsField _force true "Field_LinearVelocity" 0 (Field|SetRadialVector (Variables|Default|GetRadialVector) 1e+04 _returnvalue)))

(fn SpawnNiagara
  (bind _canon (Variables|Default|GetCanon))
  (bind _returnvalue (Transformation|GetRelativeTransform _canon))
  (Niagara|SpawnSystematLocation "/Game/BlinkAndDashVFX/VFX_Niagara/NS_Blink_Fire.NS_Blink_Fire" (.location _returnvalue) (.rotation _returnvalue) (.scale _returnvalue)))

(fn BoxTraceDetectRunningMan
  (bind _box (Variables|Default|GetBox))
  (bind _returnvalue (Transformation|GetWorldTransform _box))
  (bind _outhit (Class|KismetSystemLibrary|BoxTraceSingleforObjects (.location _returnvalue) (- (.location _returnvalue) "500.000000,0,0") (Components|Box|GetScaledBoxExtent _box) "0, 0, 0" (Variables|Default|GetObject%20Types) false 0 "ForOneFrame" true))
  (return (.hitactor _outhit)))