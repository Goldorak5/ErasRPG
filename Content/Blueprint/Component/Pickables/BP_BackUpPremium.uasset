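; BP_BackUpPremium is a pickable variant whose health value equals the player's maximum health, suggesting a full-heal backup.
; On BeginPlay it runs the parent logic, casts player 0's character to BP_RunningMan and copies HealthMax into HealthValue once.
; It adds no other active logic: its overlap and tick events are disabled, and its construction script only calls the parent.
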(event EventBeginPlay
  (|CallParentFunction)
  (bind _asbp_running_man (Utilities|Casting|CastToBP_RunningMan (Game|GetPlayerCharacter 0)))
  (Variables|Default|SetHealthValue (Variables|/Game/Blueprint/Character/RunningMan/BP_RunningMan.BP_RunningMan_C|GetHealthMax _asbp_running_man)))

(event Collision|EventActorBeginOverlap
  (params (OtherActor :type Actor%20Object%20Reference))
  (|CallParentFunction OtherActor) ; This node is disabled and will not be called.\nDrag off pins to build functionality.
)

(event EventTick
  (params (DeltaSeconds :type Float%20%28single-precision%29))
  (|CallParentFunction DeltaSeconds) ; This node is disabled and will not be called.\nDrag off pins to build functionality.
)

(fn ConstructionScript
  (|CallParentFunction))